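; Interactable phone actor for a horror scare that rings when approached and, once answered, plays a "don't turn around" voice line and toggles a monster.
; An outer RingRing trigger starts and stops a ring sound pre-spawned at the phone mesh, while an Answer trigger gates E-key input.
; Answering sets a one-shot flag that blocks further rings and calls, then toggles the monster again after a delay.
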(event `self.RingRing.OnComponentBeginOverlap`
  (params (OverlappedComponent :type "PrimitiveComponent Object Reference") (OtherActor :type "Actor Object Reference") (OtherComp :type "PrimitiveComponent Object Reference") (OtherBodyIndex :type Integer) (bFromSweep :type Boolean) (SweepResult :type "HitResult Structure (by ref)"))
  (bind _ringing (`self.ringing`))
  ;[1 1 1] play ring on enter
  (if (`AudioComponent.IsPlaying` _ringing)
    _
    (elif (not (`self.isAnswered`))
      (`AudioComponent.Play` _ringing 0.0))))

(event `Key|E`
  (params (Key :type "Key Structure"))
  ;[1 1 1] Trigger phone call and monster
  (:`Pressed`
    (if (not (`self.isAnswered`))
      (`AudioComponent.Stop` (`self.ringing`))
      (`GameplayStatics.SpawnSoundAtLocation` "/Game/audio/dont_turn_around.dont_turn_around" (`SceneComponent.K2_GetComponentLocation` (`self.SM_Phone`)) (struct) 1.0 1.0 0.0 null null)
      (set `self.isAnswered` true)
      (`/Game/blueprints/MonsterBP.toggleMonster` (`self.monster`))
      ;[1 1 1] Stop Monster
      (`KismetSystemLibrary.Delay` 8.0)
      (`/Game/blueprints/MonsterBP.toggleMonster` (`self.monster`)))))

(event `self.Answer.OnComponentBeginOverlap`
  (params (OverlappedComponent :type "PrimitiveComponent Object Reference") (OtherActor :type "Actor Object Reference") (OtherComp :type "PrimitiveComponent Object Reference") (OtherBodyIndex :type Integer) (bFromSweep :type Boolean) (SweepResult :type "HitResult Structure (by ref)"))
  ;[1 1 1] enable input for phone interaction
  (`self.EnableInput` (`GameplayStatics.GetPlayerController` 0)))

(event `self.ReceiveBeginPlay`
  ;[1 1 1] Spawn ringing
  (bind _returnvalue (`GameplayStatics.SpawnSoundAtLocation` "/Game/audio/610191__bennettfilmteacher__old-phone-ringing.610191__bennettfilmteacher__old-phone-ringing" (`SceneComponent.K2_GetComponentLocation` (`self.SM_Phone`)) (struct) 1.0 1.0 0.0 null null false))
  (bind _output_get (set `self.ringing` _returnvalue))
  (`AudioComponent.Stop` _output_get))

(event `self.Answer.OnComponentEndOverlap`
  (params (OverlappedComponent :type "PrimitiveComponent Object Reference") (OtherActor :type "Actor Object Reference") (OtherComp :type "PrimitiveComponent Object Reference") (OtherBodyIndex :type Integer))
  ;[1 1 1] enable input for phone interaction
  (`self.DisableInput` (`GameplayStatics.GetPlayerController` 0)))

(event `self.RingRing.OnComponentEndOverlap`
  (params (OverlappedComponent :type "PrimitiveComponent Object Reference") (OtherActor :type "Actor Object Reference") (OtherComp :type "PrimitiveComponent Object Reference") (OtherBodyIndex :type Integer))
  ;[1 1 1] Stop ring on leave
  (`AudioComponent.Stop` (`self.ringing`)))

(fn `UserConstructionScript`)