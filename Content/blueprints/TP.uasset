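; TP is a paper towel roll pickup that opens a referenced Door when collected.
; A Box overlap volume enables and disables the actor's input for player controller 0, so E only responds within range.
; Pressing E calls OpenDoor on the Door, plays a pickup sound at the roll's location and destroys the actor.
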(event `Key|E`
  (params (Key :type "Key Structure"))
  (:`Pressed`
    (`/Game/blueprints/DoorOpenBP.Open Door` (`self.door`))
    (`GameplayStatics.PlaySoundAtLocation` "/Game/audio/509879__slamaxu__pickup_generic.509879__slamaxu__pickup_generic" (`SceneComponent.K2_GetComponentLocation` (`self.S_Paper_Towel_Roll_vh3pbe2s_lod3`)) (struct) 1.0 1.0 0.0 null null null null)
    (`self.K2_DestroyActor`)))

(event `self.Box.OnComponentBeginOverlap`
  (params (OverlappedComponent :type "PrimitiveComponent Object Reference") (OtherActor :type "Actor Object Reference") (OtherComp :type "PrimitiveComponent Object Reference") (OtherBodyIndex :type Integer) (bFromSweep :type Boolean) (SweepResult :type "HitResult Structure (by ref)"))
  ;[1 1 1] Enable and disable input
  (`self.EnableInput` (`GameplayStatics.GetPlayerController` 0)))

(event `self.Box.OnComponentEndOverlap`
  (params (OverlappedComponent :type "PrimitiveComponent Object Reference") (OtherActor :type "Actor Object Reference") (OtherComp :type "PrimitiveComponent Object Reference") (OtherBodyIndex :type Integer))
  ;[1 1 1] Enable and disable input
  (`self.DisableInput` (`GameplayStatics.GetPlayerController` 0)))

(fn `UserConstructionScript`)