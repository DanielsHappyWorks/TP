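; Flickering light actor that animates a light's intensity when something overlaps its Box trigger.
; BeginPlay caches the light's original intensity, which the Flicker timeline's track scales from zero via Lerp.
; Each timeline update also sets IsPlaying and plays the flicker sound at the light's location.
; IsPlaying is never cleared here, so later overlaps do not replay the timeline.
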(event `self.Box.OnComponentBeginOverlap`
  (params (OverlappedComponent :type "PrimitiveComponent Object Reference") (OtherActor :type "Actor Object Reference") (OtherComp :type "PrimitiveComponent Object Reference") (OtherBodyIndex :type Integer) (bFromSweep :type Boolean) (SweepResult :type "HitResult Structure (by ref)"))
  ;[1 1 1] flicker based on timeline and lerp
  (if (not (`self.isPlaying`))
    (bind (_direction _newtrack_0) (`Timeline|flicker`)
      (:`Update`
        (`LightComponent.SetIntensity` (`Light.LightComponent` (`self.light`)) (`KismetMathLibrary.Lerp` 0.0 (`self.intensity`) _newtrack_0))
        (set `self.isPlaying` true)
        (`GameplayStatics.PlaySoundAtLocation` "/Game/audio/111625__kiefspoon__flickering-light-de-noised.111625__kiefspoon__flickering-light-de-noised" (`SceneComponent.K2_GetComponentLocation` (`Light.LightComponent` (`self.light`))) (struct) 1.0 1.0 0.0 null null null null)))))

(event `self.ReceiveBeginPlay`
  ;[1 1 1] copy original intensity
  (set `self.intensity` (`LightComponentBase.Intensity` (`Light.LightComponent` (`self.light`)))))

(fn `UserConstructionScript`)