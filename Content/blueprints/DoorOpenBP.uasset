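; Interactive restroom cabin door actor that the player swings open or closed with the E key.
; A box overlap enables input only while something is inside it, and E plays or reverses a Timeline based on IsOpen.
; The Timeline drives the actor's absolute yaw and plays a creak sound once per swing, then flips IsOpen and resets the sound guard on finish.
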(event `Key|E`
  (params (Key :type "Key Structure"))
  (bind _isopen (`self.isOpen`))
  (:`Pressed`
    (if _isopen
      (bind (_direction _open) (`Timeline|Timeline` :!via `Reverse` :!label _label)
        (:`Update`
          (`self.K2_SetActorRotation` (`KismetMathLibrary.MakeRotator` 0.0 0.0 _open))
          (if (not (`self.isPlayingCreek`))
            (`GameplayStatics.PlaySoundAtLocation` "/Game/audio/702171__foxfire__door-opening.702171__foxfire__door-opening" (`SceneComponent.K2_GetComponentLocation` (`self.SM_RestroomCabinDoor`)) (struct) 1.0 1.0 0.0 null null null null)
            (set `self.isPlayingCreek` true)))
        (:`Finished`
          (set `self.isOpen` (not _isopen))
          (set `self.isPlayingCreek` false)))
      (else
        (goto _label)))))

(event `self.Box.OnComponentBeginOverlap`
  (params (OverlappedComponent :type "PrimitiveComponent Object Reference") (OtherActor :type "Actor Object Reference") (OtherComp :type "PrimitiveComponent Object Reference") (OtherBodyIndex :type Integer) (bFromSweep :type Boolean) (SweepResult :type "HitResult Structure (by ref)"))
  (`self.EnableInput` (`GameplayStatics.GetPlayerController` 0)))

(event `self.Box.OnComponentEndOverlap`
  (params (OverlappedComponent :type "PrimitiveComponent Object Reference") (OtherActor :type "Actor Object Reference") (OtherComp :type "PrimitiveComponent Object Reference") (OtherBodyIndex :type Integer))
  (`self.DisableInput` (`GameplayStatics.GetPlayerController` 0)))

(fn `UserConstructionScript`)